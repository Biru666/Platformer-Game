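; Game mode for the platformer that handles the win sequence.
; Its Win event disables player character input and fades the camera toward a mostly opaque white, holding the fade.
; After a delay matching the fade, it creates the Final_Screen widget, adds it to the viewport, switches to UI-only input and shows the mouse cursor.
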(event Custom|Win
  (bind _returnvalue (Game|GetPlayerController 0))
  (Input|DisableInput (Game|GetPlayerCharacter 0) (Game|GetPlayerController 0))
  (CameraFades|StartCameraFade (Game|GetPlayerCameraManager 0) 0.0 0.8 2.0 "(R=1.000000,G=1.000000,B=1.000000,A=1.000000)" false true)
  (Utilities|FlowControl|Delay 2.0)
  (bind _returnvalue_2 (UserInterface|CreateWidget "/Game/Platformer/HUD/Final_Screen.Final_Screen_C"))
  (UserInterface|Viewport|AddtoViewport _returnvalue_2 0)
  (Input|SetInputModeUIOnly _returnvalue 0 "DoNotLock")
  (Variables|/Script/Engine.PlayerController|SetbShowMouseCursor _returnvalue true))

(fn ConstructionScript)