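; BP_AI is a platformer AI character with a flipbook sprite that walks back and forth along the X axis.
; Each Tick adds movement input in the current direction and yaws the sprite 0 or 180 degrees to match IsMovingRight.
; Any capsule hit toggles IsMovingRight, reversing the patrol without navigation or a behavior tree.
; The velocity-based animation update selects the Walk flipbook whether moving or stationary.
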(event OnComponentHit(CapsuleComponent)
  (params (HitComponent :type Primitive%20Component%20Object%20Reference) (OtherActor :type Actor%20Object%20Reference) (OtherComp :type Primitive%20Component%20Object%20Reference) (NormalImpulse :type Vector :default "0, 0, 0") (Hit :type Hit%20Result%20Structure%20%28by%20ref%29))
  (Variables|Default|SetisMovingRight (not (Variables|Default|GetisMovingRight))))

(event Custom|Direction
  ;[1 1 1] Direction flip
  (Transformation|SetRelativeRotation (Variables|Default|GetSprite) (Math|Rotator|MakeRotator 0.0 0.0 (Math|Float|SelectFloat 0.0 1.8e+02 (Variables|Default|GetisMovingRight))) false false)
  (Pawn|Input|AddMovementInput (Math|Vector|SelectVector "1.000000, 0, 0" "-1.000000, 0, 0" (Variables|Default|GetisMovingRight)) 1.0 false))

(event Custom|UpdateAnimation
  ;[1 1 1] Handle Animation
  (Sprite|SetFlipbook (Variables|Default|GetSprite) (select (> (Math|Vector|VectorLength (Transformation|GetVelocity)) 0.0) "/Game/Platformer/Sprites/AI/walk.walk" "/Game/Platformer/Sprites/AI/walk.walk")))

(event EventTick
  (params (DeltaSeconds :type Float%20%28single-precision%29))
  (CallFunction|Direction)
  (CallFunction|UpdateAnimation))

(fn ConstructionScript)