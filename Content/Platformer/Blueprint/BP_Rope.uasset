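; BP_Rope is a climbable rope actor for a platformer, moving the player upward while Q is held.
; Tick measures and prints the player's X offset from the rope, sets IsOnRope within a narrow band, and enables input in either case.
; Pressing Q starts a Delay-based polling loop that sets Flying and adds upward movement input, restoring Walking when Q is released or the player is off the rope.
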(event Collision|EventActorBeginOverlap
  (params (OtherActor :type Actor%20Object%20Reference)))

(event EventTick
  (params (DeltaSeconds :type Float%20%28single-precision%29))
  (bind _returnvalue (Game|GetPlayerController 0))
  (Utilities|FlowControl|Sequence
    (:then_0
      (Variables|Default|SetDisRope (- (.x (Transformation|GetActorLocation (Game|GetPlayerCharacter 0))) (.x (Transformation|GetActorLocation)))))
    (:then_1
      (Development|PrintString (Utilities|String|ToString(Float) (Variables|Default|GetDisRope))))
    (:then_2
      (if (Math|Float|InRange(Float) (Variables|Default|GetDisRope) -5.0 5.0 false)
        (Variables|Default|SetisOnRope true)
        (Input|EnableInput _returnvalue)
        (else
          (Variables|Default|SetisOnRope false)
          (Input|EnableInput _returnvalue))))))

(event Input|KeyboardEvents|Q
  (params (Key :type Key%20Structure :default "None"))
  (bind _returnvalue (Game|Player|GetPlayerPawn 0))
  (:Pressed
    (if (Variables|Default|GetisOnRope) :!label _label
      (if (Game|Player|IsInputKeyDown (Game|GetPlayerController 0) "Q")
        (Pawn|Components|CharacterMovement|SetMovementMode (Variables|/Script/Engine.Character|GetCharacterMovement (Game|GetPlayerCharacter 0)) "MOVE_Flying" 0)
        (Pawn|Input|AddMovementInput _returnvalue (Transformation|GetActorUpVector _returnvalue) (Variables|Default|GetMovementSpeed) false)
        (Utilities|FlowControl|Delay 0.2)
        (goto _label)
        (else
          _)))
    (Pawn|Components|CharacterMovement|SetMovementMode (Variables|/Script/Engine.Character|GetCharacterMovement (Game|GetPlayerCharacter 0)) "MOVE_Walking" 0)))

(fn ConstructionScript)